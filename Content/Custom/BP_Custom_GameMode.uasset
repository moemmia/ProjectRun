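; Game mode for an endless-runner style loop that scrolls randomly chosen tiles along the world forward axis.
; StartEvent hides the menu and starts a looping timer that spawns tiles at SpawnPoint, while EndEvent stops it and restores the menu.
; Tick moves tiles by a per-frame offset, removes the oldest using a dot-product check against DespawnPoint, and tracks play time.
; When not playing, Tick destroys all remaining tiles.
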(event Custom|Spawn%20Tiles
  (CallFunction|SpawnRandomTile))

(event Custom|StartEvent
  (params (Actor :type Widget%20Object%20Reference))
  (bind _output_get (Variables|Default|SetMainMenu Actor))
  (Widget|SetVisibility _output_get "Hidden")
  (bind _returnvalue (Utilities|Time|SetTimerbyEvent (delegate Custom|Spawn%20Tiles) (Variables|Default|GetSpawn%20Velocity) true 0.1))
  (Variables|Default|SetSpawnTimer _returnvalue)
  (Variables|Default|SetPlaying true)
  (Variables|Default|SetTimeOnStart (Math|Float|Truncate (Utilities|Time|GetRealTimeSeconds))))

(event Custom|EndEvent
  (Variables|Default|SetPlaying false)
  (Utilities|Time|ClearandInvalidateTimerbyHandle (Variables|Default|GetSpawnTimer))
  (Widget|SetVisibility (Variables|Default|GetMainMenu) "Visible")
  (Variables|Default|SetTimeOnPlay 0))

(event EventTick
  (params (DeltaSeconds :type Float%20%28single-precision%29))
  (bind _spawnedtilelist (Variables|Default|GetSpawnedTileList))
  (bind _spawnedtilelist_2 (Variables|Default|GetSpawnedTileList))
  (bind _returnvalue (Utilities|Array|Length _spawnedtilelist_2))
  (bind _output (Utilities|Array|Get(acopy) _spawnedtilelist))
  (Utilities|FlowControl|Sequence
    (:then_0
      (if (Variables|Default|GetPlaying)
        (for _array_element _spawnedtilelist
          (Utilities|IsValid _array_element
            (:Is%20Valid
              (Transformation|AddActorWorldOffset _array_element (* (Class|KismetMathLibrary|VectorForward) (Variables|Default|GetActors%20Velocity))))))
        (Utilities|IsValid _output
          (:Is%20Valid
            (if (< (Math|Vector|DotProduct (Math|Vector|Normalize (- (Transformation|GetActorLocation _output) (Variables|Default|GetDespawnPoint))) (Class|KismetMathLibrary|VectorForward)) 0.0)
              (Actor|DestroyActor _output)
              (Utilities|Array|RemoveIndex (Variables|Default|GetSpawnedTileList)))))
        (elif (> _returnvalue 0)
          (Variables|Default|SetTMP_Counter _returnvalue)
          (while (> (Variables|Default|GetTMP_Counter) 0)
            (bind _result (Math|Integer|DecrementInt (Variables|Default|GetTMP_Counter))
              (:%20%20
                (Actor|DestroyActor (Utilities|Array|Get(acopy) (Variables|Default|GetSpawnedTileList) _result)))))
          (Utilities|Array|Clear (Variables|Default|GetSpawnedTileList)))))
    (:then_1
      (if (Variables|Default|GetPlaying)
        (Variables|Default|SetTimeOnPlay (- (Math|Float|Truncate (Utilities|Time|GetRealTimeSeconds)) (Variables|Default|GetTimeOnStart)))))))

(fn ConstructionScript)

(fn SpawnRandomTile
  (bind _returnvalue (Game|SpawnActorfromClass (Utilities|Array|Get(acopy) (Variables|Default|GetTileList) (Math|Random|RandomIntegerinRange 0 (- (Utilities|Array|Length (Variables|Default|GetTileList)) 1))) (Variables|Default|GetSpawnPoint) "Undefined" 0 0))
  (Utilities|Array|Add (Variables|Default|GetSpawnedTileList) _returnvalue))